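; BP_ModActor is an actor that integrates a mod with the ModLoader, apparently as a base class with stub functions for config, deactivation and widget opening.
; It binds to the loader's init, shutdown and load-data dispatches and forwards log messages to it.
; When settings are enabled, it saves to a per-mod slot, then reloads and copies entries into its own and the loader's config.
; Its construction script can enforce a singleton.
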(event `self.BindEvents`
  (bind _modloader (`self.ModLoader`))
  (add `/FF7RML/ModLoaders/BP_FF7RModLoader_Base.PostInitDispatch` _modloader (`|CreateDelegate` :!event `PostInit`))
  (add `/FF7RML/ModLoaders/BP_FF7RModLoader_Base.PostGameInstanceInitDispatch` _modloader (`|CreateDelegate` :!event `PostGameInstanceInit`))
  (add `/FF7RML/ModLoaders/BP_FF7RModLoader_Base.ShutdownDispatch` _modloader (`|CreateDelegate` :!event `Shutdown`))
  (add `/FF7RML/ModLoaders/BP_FF7RModLoader_Base.LoadDataDispatch` _modloader (`|CreateDelegate` :!event `LoadData`)))

(event `self.PrintToModLoader`
  (params (Message :type String))
  (`/FF7RML/ModLoaders/BP_FF7RModLoader.LogPrintToModLoaderImpl` (`self.ModLoader`) Message self))

(event `self.SaveData`
  (params (InSave :type "EndSaveGame Object Reference"))
  (if (`self.HasSettings`)
    (`GameplayStatics.SaveGameToSlot` InSave (`KismetStringLibrary.Concat_StrStr` "ModConfig_" (`KismetStringLibrary.Conv_NameToString` (`self.ModName`))))
    (`self.LoadData`)))

(event `self.LoadData`
  (if (`self.HasSettings`)
    (bind _returnvalue (`GameplayStatics.LoadGameFromSlot` (`KismetStringLibrary.Concat_StrStr` "ModConfig_" (`KismetStringLibrary.Conv_NameToString` (`self.ModName`)))))
    (bind _asbp_mod_save_game (cast `/FF7RML/Classes/BP_ModSaveGame` _returnvalue))
    (bind _modconfigsavedata (`/FF7RML/Classes/BP_ModSaveGame.ModConfigSaveData` _asbp_mod_save_game))
    (bind _keys (`BlueprintMapLibrary.Map_Keys` _modconfigsavedata))
    (for _array_element _keys
      (bind _value (`BlueprintMapLibrary.Map_Find` _modconfigsavedata _array_element))
      (`BlueprintMapLibrary.Map_Add` (`/FF7RML/ModLoaders/Structs/PDA_ModConfig.ModConfiguration` (`self.ModConfig`)) _array_element _value)
      (`BlueprintMapLibrary.Map_Add` (`/FF7RML/ModLoaders/Structs/PDA_ModConfig.ModConfiguration` (`BlueprintMapLibrary.Map_Find` (`/FF7RML/ModLoaders/BP_FF7RModLoader.ModConfig` (`self.ModLoader`)) (`self.ModName`))) _array_element _value))))

(fn `GetConfig`
  (returns (Config :type "/FF7RML/Classes/BP_ModSaveGame Object Reference"))
  (return null))

(fn `IsDeactivated`
  (returns (Deactivated :type Boolean))
  (return false))

(fn `OpenWidget`
  (returns (Success :type Boolean))
  (return false))

(fn `UserConstructionScript`
  (if (`self.bEnsureSingleton`)
    (bind _returnvalue (`GameplayStatics.GetActorOfClass` (`GameplayStatics.GetObjectClass` self)))
    (if (!= _returnvalue self)
      (`self.K2_DestroyActor`))))