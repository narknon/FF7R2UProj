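; Base mod object class that hooks into the ModLoader lifecycle and logs to it.
; BindEvents registers handlers for the loader's pre-init, init, post-init, post-game-instance-init, shutdown and load-data dispatches.
; PrinttoModLoader forwards messages to the loader with itself as source when the loader is valid.
; GetConfig is empty, and a binding log message sits on an unreached path.
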(event `/FF7RML/Interfaces/BPI_Mods.BindEvents`
  (bind _modloader (`self.ModLoader`))
  (add `/FF7RML/ModLoaders/BP_FF7RModLoader_Base.PreInitDispatch` _modloader (`|CreateDelegate` :!event `PreInit`))
  (add `/FF7RML/ModLoaders/BP_FF7RModLoader_Base.InitDispatch` _modloader (`|CreateDelegate` :!event `Init`))
  (add `/FF7RML/ModLoaders/BP_FF7RModLoader_Base.PostInitDispatch` _modloader (`|CreateDelegate` :!event `PostInit`))
  (add `/FF7RML/ModLoaders/BP_FF7RModLoader_Base.PostGameInstanceInitDispatch` _modloader (`|CreateDelegate` :!event `PostGameInstanceInit`))
  (add `/FF7RML/ModLoaders/BP_FF7RModLoader_Base.ShutdownDispatch` _modloader (`|CreateDelegate` :!event `Shutdown`))
  (add `/FF7RML/ModLoaders/BP_FF7RModLoader_Base.LoadDataDispatch` _modloader (`|CreateDelegate` :!event `LoadData`)))

(event `/FF7RML/Interfaces/BPI_Mods.PrintToModLoader`
  (params (Message :type String))
  (bind _modloader (`self.ModLoader`))
  (`/Engine/EditorBlueprintResources/StandardMacros.IsValid` _modloader
    (:`Is Valid`
      (`/FF7RML/ModLoaders/BP_FF7RModLoader.LogPrintToModLoaderImpl` _modloader Message self))))

(fn `GetConfig`
  (returns (Config :type "/FF7RML/Classes/BP_ModSaveGame Object Reference"))
  (return null))