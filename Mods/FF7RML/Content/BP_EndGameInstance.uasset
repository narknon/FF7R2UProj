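; BP_EndGameInstance is a game instance that bootstraps and shuts down a mod loader.
; On Init it constructs the loader from ModLoaderClass with itself as outer and calls PreInit and Init.
; After a zero-length Delay it calls PostInit, hands the loader a reference to itself and calls PostGameInstanceInit.
; Shutdown forwards to the loader's own Shutdown.
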(event `self.ReceiveInit`
  (bind _modloader (`self.ModLoader`))
  (`/FF7RML/FunctionLibs/BPFL_FF7RModLoader.PrintToModLoader` "PreLoadML")
  (bind _returnvalue (`|GenericCreateObject` (`self.ModLoaderClass`) self null))
  (bind _output_get (set `self.ModLoader` _returnvalue))
  (`/FF7RML/ModLoaders/BP_FF7RModLoader_Base.PreInit` _output_get)
  (`/FF7RML/ModLoaders/BP_FF7RModLoader_Base.Init` (`self.ModLoader`))
  (`KismetSystemLibrary.Delay` 0.0)
  (`/FF7RML/ModLoaders/BP_FF7RModLoader_Base.PostInit` (`self.ModLoader`))
  (set `/FF7RML/ModLoaders/BP_FF7RModLoader.GameInstace` self _modloader)
  (`/FF7RML/Interfaces/BPI_Mods.PostGameInstanceInit` _modloader))

(event `self.ReceiveShutdown`
  (`/FF7RML/Interfaces/BPI_Mods.Shutdown` (`self.ModLoader`)))