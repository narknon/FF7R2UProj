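; Mod loader extension that discovers PDA_DynamicDA data assets and merges their character (costume) data into its own map.
; LoadDAs scans every Asset Registry entry outside FF7RML paths, blocking-loads each and casts it to PDA_DynamicDA.
; Matches are recorded in DynamicDAsFound, and IterateCostumeData copies their key/value pairs into CharacterData, logging to the mod loader.
; PreInit and Init are empty, and nothing here calls LoadDAs.
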(event `/FF7RML/Interfaces/BPI_ModObjects.PreInit`)

(event `/FF7RML/Interfaces/BPI_ModObjects.Init`)

(fn `IterateCostumeData`
  (params (TargetMap :type "Map of Name to /FF7RML/ModLoaders/Extensions/DynamicAsset/Structs/UDS_CharacterSubData Structure"))
  (bind _characterdata_characterdata (break `/FF7RML/ModLoaders/Extensions/DynamicAsset/Structs/UDS_CharacterData` (`self.CharacterData`)))
  (bind _keys (`BlueprintMapLibrary.Map_Keys` TargetMap))
  (for _array_element _keys
    (`self.PrintToModLoader` (`KismetStringLibrary.Concat_StrStr` "Adding Key:" (`KismetStringLibrary.Conv_NameToString` _array_element)))
    (`BlueprintMapLibrary.Map_Add` _characterdata_characterdata _array_element (`BlueprintMapLibrary.Map_Find` (`local.TargetMap`) _array_element))))

(fn `LoadDAs`
  (bind _outassetdata (`AssetRegistry.GetAllAssets` (`AssetRegistryHelpers.GetAssetRegistry`) false))
  (for _array_element _outassetdata
    (bind (_objectpath _packagename _packagepath _assetname) (break `AssetData` _array_element))
    (if (not (`KismetStringLibrary.Contains` (`KismetStringLibrary.Conv_NameToString` _packagepath) "FF7RML"))
      (bind _returnvalue (`KismetStringLibrary.Concat_StrStr` (`KismetStringLibrary.Conv_NameToString` _packagename) "." (`KismetStringLibrary.Conv_NameToString` _assetname)))
      (`/FF7RML/FunctionLibs/BPFL_FF7RModLoader.PrintToModLoader` (`KismetStringLibrary.Concat_StrStr` "Found Dynamic DA:" _returnvalue))
      (bind _returnvalue_2 (`KismetSystemLibrary.LoadAsset_Blocking` (`KismetSystemLibrary.Conv_SoftObjPathToSoftObjRef` (`KismetSystemLibrary.MakeSoftObjectPath` _returnvalue))))
      (bind _aspda_dynamic_da (cast `/FF7RML/ModLoaders/Extensions/DynamicAsset/Structs/PDA_DynamicDA` _returnvalue_2))
      (`KismetArrayLibrary.Array_Add` (`self.DynamicDAsFound`) _array_element)
      (`|ExecutionSequence`
        (:`then_0`
          (`self.IterateCostumeData` (`.CharacterData_13_5D7C69B8438D2B428F93F1B48C9AD3F8` (break `/FF7RML/ModLoaders/Extensions/DynamicAsset/Structs/UDS_CharacterData` (`/FF7RML/ModLoaders/Extensions/DynamicAsset/Structs/PDA_DynamicDA.CharacterData` _aspda_dynamic_da)))))))))