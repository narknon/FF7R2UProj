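; Base Blueprint for an FF7R mod loader, providing helpers for debug output and mod metadata lookup.
; Debug printing reuses a valid local widget, falls back to the mod loader's shared one, or constructs a new one on demand.
; Mod names come from the first segment of a path and build a soft path to each mod's metadata data asset, which loads synchronously.
; GetConfig is an empty stub.
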(fn `ConstructDebugWidget`
  (params (InString :type String) (InTitle :type String))
  (returns (NewDebugWidget :type "/FF7RML/UI/WBP_DebugWidget Object Reference"))
  (bind _returnvalue (`|GenericCreateObject` (`self.DebugWidgetClass`) self InString InTitle))
  (`self.AddToViewport` _returnvalue 0)
  (return _returnvalue))

(fn `GetConfig`
  (returns (Config :type "/FF7RML/Classes/BP_ModSaveGame Object Reference"))
  (return null))

(fn `GetMetaDataDA`
  (params (ModName :type Name))
  (returns (DA_MetaData :type "/FF7RML/ModLoaders/Structs/UDS_ModMetaData Structure"))
  (bind _returnvalue (`KismetSystemLibrary.LoadAsset_Blocking` (`KismetSystemLibrary.Conv_SoftObjPathToSoftObjRef` (`KismetSystemLibrary.MakeSoftObjectPath` (`KismetStringLibrary.Concat_StrStr` "/" (`KismetStringLibrary.Conv_NameToString` ModName) "/" "MetaData/" "DA_ModMetaData.DA_ModMetaData")))))
  (bind _aspda_mod_meta_data (cast `/FF7RML/ModLoaders/Structs/PDA_ModMetaData` _returnvalue))
  (return (`/FF7RML/ModLoaders/Structs/PDA_ModMetaData.MetaData` _aspda_mod_meta_data)))

(fn `GetModNameFromPath`
  (params (SourceString :type String))
  (returns (ReturnValue :type Name))
  (return (`KismetStringLibrary.Conv_StringToName` (`|GetArrayItem` (`KismetStringLibrary.ParseIntoArray` SourceString "/")))))

(fn `PrintToDebugWidget`
  (params (Title :type String) (Message :type String) (bNewWindow :type Boolean))
  (returns (DebugWidget :type "/FF7RML/UI/WBP_DebugWidget Object Reference"))
  (bind _debugwidget (`self.DebugWidget`))
  (bind _debugwidget_2 (`/Game/ModLoaders/BP_FF7RModLoader_Base.DebugWidget` (`/FF7RML/FunctionLibs/BPFL_FF7RModLoader.GetModLoader`)))
  (if bNewWindow
    (bind _newdebugwidget (`self.ConstructDebugWidget` Title Message :!label _label))
    (set `self.DebugWidget` _newdebugwidget)
    (else
      (`/Engine/EditorBlueprintResources/StandardMacros.IsValid` _debugwidget
        (:`Is Valid`
          _)
        (:`Is Not Valid`
          (`/Engine/EditorBlueprintResources/StandardMacros.IsValid` _debugwidget_2
            (:`Is Valid`
              (set `self.DebugWidget` _debugwidget_2))
            (:`Is Not Valid`
              (goto _label)))))
      (`/FF7RML/UI/WBP_DebugWidget.PrintTextFromString` _debugwidget (`local.Message`))
      (`self.SetVisibility` _debugwidget "Visible")))
  (return (`self.DebugWidget`)))