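; Base Blueprint for FF7R mod loader extensions, giving each mod lifecycle hooks and a logging helper.
; BindEvents registers handlers with the ModLoader's PreInit, Init, PostInit, PostGameInstanceInit and Shutdown dispatchers.
; PrinttoModLoader prefixes messages with the mod name derived from the object's class path and forwards them to the loader's log.
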(event `/FF7RML/Interfaces/BPI_Mods.BindEvents`
  (add `self.PreInitDispatch` (`self.ModLoader`) (`|CreateDelegate` :!event `PreInit`))
  (add `self.InitDispatch` (`self.ModLoader`) (`|CreateDelegate` :!event `Init`))
  (add `self.PostInitDispatch` (`self.ModLoader`) (`|CreateDelegate` :!event `PostInit`))
  (add `self.PostGameInstanceInitDispatch` (`self.ModLoader`) (`|CreateDelegate` :!event `PostGameInstanceInit`))
  (add `self.ShutdownDispatch` (`self.ModLoader`) (`|CreateDelegate` :!event `Shutdown`)))

(event `/FF7RML/Interfaces/BPI_Mods.PrintToModLoader`
  (params (Message :type String))
  (`/FF7RML/ModLoaders/BP_FF7RModLoader.LogPrintToModLoaderImpl` (`self.ModLoader`) (`KismetStringLibrary.Concat_StrStr` "[" (`KismetStringLibrary.Conv_NameToString` (`self.GetModNameFromPath` (`KismetSystemLibrary.Conv_SoftClassReferenceToString` (`|ConvertAsset` (`GameplayStatics.GetObjectClass` self))))) "]: " Message) self))