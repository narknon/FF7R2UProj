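; Actor for an FF7R mod that opens the mod menu from keyboard or gamepad.
; It enables input on BeginPlay, then listens for F8 or times both thumbsticks held down on Tick against a HoldTime read from the mod loader's FF7RModMenu config.
; Both triggers share one path that, unless the menu is already visible, constructs a new WBP_ModMenu_Base, focuses it and adds it to the viewport.
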(event `/FF7RML/Interfaces/BPI_Mods.PostInit`)

(event `self.ReceiveBeginPlay`
  (`parent.ReceiveBeginPlay`)
  (`self.EnableInput` (`GameplayStatics.GetPlayerController` 0)))

(event `Key|+`
  (params (Key :type "Key Structure")))

(event `Key|F8`
  (params (Key :type "Key Structure"))
  (:`Pressed`
    (if (not (`Widget.IsVisible` (`self.ModMenu`))) :!label _label
      (bind _returnvalue (`|GenericCreateObject` "/FF7RModMenu/UI/WBP_ModMenu_Base.WBP_ModMenu_Base_C" (`GameplayStatics.GetGameInstance`)))
      (bind _output_get (set `self.ModMenu` _returnvalue))
      (`EndMenuAPI.SetFocusToWidget` _output_get)
      (`UserWidget.AddToViewport` _output_get 0))))

(event `self.ReceiveTick`
  (params (DeltaSeconds :type "Float (single-precision)"))
  (`parent.ReceiveTick` DeltaSeconds)
  (bind _returnvalue (`EndSystemAPI.IsInputKeyDown` "Gamepad_LeftThumbstick"))
  (bind _returnvalue_2 (`EndSystemAPI.IsInputKeyDown` "Gamepad_RightThumbstick"))
  (if (and _returnvalue _returnvalue_2)
    (bind _output_get (set `self.HoldTimer` (+ DeltaSeconds (`self.HoldTimer`))))
    (if (> _output_get (`self.GetHoldTime`))
      (goto _label))
    (else
      (set `self.HoldTimer` 0.0))))

(fn `GetHoldTime`
  (returns (HoldTime :type "Float (double-precision)"))
  (return (`.DefaultFloat_17_D230CC244231AF05217ABDAE32E5A77E` (break `/FF7RML/ModLoaders/Structs/UDS_ModConfigOption` (`BlueprintMapLibrary.Map_Find` (`/FF7RML/ModLoaders/Structs/PDA_ModConfig.ModConfiguration` (`BlueprintMapLibrary.Map_Find` (`/FF7RML/ModLoaders/BP_FF7RModLoader.ModConfig` (`/FF7RML/FunctionLibs/BPFL_FF7RModLoader.GetModLoader`)) "FF7RModMenu")) "HoldTime")))))

(fn `UserConstructionScript`
  (`parent.UserConstructionScript`))